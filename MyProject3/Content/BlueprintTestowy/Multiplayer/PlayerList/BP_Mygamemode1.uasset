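; Multiplayer game mode that runs the lobby, match start and end-of-match results.
; It tracks player controllers and ready flags, pushes updates to each client and admits joiners only while Gra is true.
; Starting clears Gra, sends non-host players to the level and pre-counts the host as finished.
; Finishers wait until all report, then GameInstance quicksorts them and everyone gets the lobby and results table.
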(event Custom|wysłanie%20do%20serwera
  (params (ThisPlayerControler :type BP%20My%20Player%20Controler%20Object%20Reference))
  (bind _all_end_playercontrolers (Variables|Default|GetAll_End_PlayerControlers))
  (bind _all_end_playercontrolers_2 (Variables|Default|GetAll_End_PlayerControlers))
  (bind _all_playercontrolers (Variables|Default|GetAll_PlayerControlers))
  (Utilities|Array|Add _all_end_playercontrolers ThisPlayerControler)
  (if (== (Utilities|Array|Length (Variables|Default|GetAll_PlayerControlers)) (Utilities|Array|Length _all_end_playercontrolers))
    (for _array_element _all_end_playercontrolers
      (Default|PobranieZInstancji _array_element)
      (Development|PrintString (Utilities|String|ToString(Float) (Utilities|Struct|BreakS_Tabela_Wyników (Variables|/Game/BlueprintTestowy/Multiplayer/PlayerList/BP_MyPlayerControler.BP_MyPlayerControler_C|GetEnd_wynik _array_element))) true true "(R=0.007224,G=0.000000,B=1.000000,A=1.000000)" 12.0 "listen"))
    (bind _asbp_game_instance_2 (Utilities|Casting|CastToBp_GameInstance2 (Game|GetGameInstance)))
    (Default|QuickSortBPMyPlayerControler _asbp_game_instance_2 _all_end_playercontrolers_2)
    (Utilities|Array|Clear (Variables|Default|GetWyniki))
    (for _array_element_2 _all_end_playercontrolers_2
      (Utilities|Array|Add (Variables|Default|GetWyniki) (Variables|/Game/BlueprintTestowy/Multiplayer/PlayerList/BP_MyPlayerControler.BP_MyPlayerControler_C|GetEnd_wynik _array_element_2)))
    (for _array_element_3 _all_playercontrolers
      (Default|ChangeMape _array_element_3)
      (Default|CreateLobbyMenu _array_element_3)
      (Default|CreateEndPlaylist _array_element_3 (Variables|Default|GetAll_End_PlayerControlers) (Utilities|Array|Get(acopy) _all_playercontrolers) (Variables|Default|GetWyniki)))
    (else
      (Default|EkranPoczekalniPoRozgrywce ThisPlayerControler))))

(event Custom|start_play
  (bind _all_playercontrolers (Variables|Default|GetAll_PlayerControlers))
  (bind _output (Utilities|Array|Get(acopy) _all_playercontrolers))
  ;[1 1 1] Start game
  (Variables|Default|Setgra false)
  (for (_array_element _array_index) _all_playercontrolers
    (if (!= _array_index 0)
      (bind _asbp_game_instance_2 (Utilities|Casting|CastToBp_GameInstance2 (Game|GetGameInstance)))
      (Default|ChaingeLevel _array_element (Variables|/Game/BlueprintTestowy/SaveData/Bp_GameInstance2.Bp_GameInstance2_C|Getmuzyka _asbp_game_instance_2))))
  (Utilities|Array|Add (Variables|Default|GetAll_End_PlayerControlers) _output)
  (Default|CreateWidgetSerwer _output))

(event Custom|UpdateLobby
  (params (Player%20Names :type Boolean) (PlayersReady :type Boolean))
  (Utilities|Array|Clear (Variables|Default|GetAll_PlayerProfiles))
  (for _array_element (Variables|Default|GetAll_PlayerControlers)
    (Utilities|Array|Add (Variables|Default|GetAll_PlayerProfiles) (Variables|/Game/BlueprintTestowy/Multiplayer/PlayerList/BP_MyPlayerControler.BP_MyPlayerControler_C|GetPlayer_Profile_Info _array_element)))
  (for _array_element_2 (Variables|Default|GetAll_PlayerControlers)
    (if Player%20Names
      (Default|UpdatePlayerNames _array_element_2 (Variables|Default|GetAll_PlayerProfiles)))
    (if PlayersReady
      (Default|UpdatePlayerReady _array_element_2 (Variables|Default|GetIsPlayerRedy)))
    (if true
      _)))

(event Custom|SetPlayerReady
  (params (PlayerController :type BP%20My%20Player%20Controler%20Object%20Reference) (IsReady :type Boolean))
  ;[1 1 1] Set Ready for player
  (Utilities|Array|SetArrayElem (Variables|Default|GetIsPlayerRedy) (Utilities|Array|FindItem (Variables|Default|GetAll_PlayerControlers) PlayerController) IsReady)
  (CallFunction|UpdateLobby false true))

(event Custom|update_end_panel)

(event EventBeginPlay)

(event EventHandleStartingNewPlayer
  (params (NewPlayer :type Player%20Controller%20Object%20Reference))
  (bind _all_playercontrolers (Variables|Default|GetAll_PlayerControlers))
  ;[1 1 1] Comment
  (if (Variables|Default|Getgra)
    (bind _returnvalue (Game|GetCurrentLevelName true))
    (switch string _returnvalue
      (:testowy_multi
        (bind _asbp_my_player_controler (Utilities|Casting|CastToBP_MyPlayerControler NewPlayer))
        (bind _returnvalue_2 (Utilities|Array|Add _all_playercontrolers _asbp_my_player_controler))
        (Variables|/Game/BlueprintTestowy/Multiplayer/PlayerList/BP_MyPlayerControler.BP_MyPlayerControler_C|SetId _asbp_my_player_controler _returnvalue_2)
        (Utilities|Array|SetArrayElem (Variables|Default|GetIsPlayerRedy) _returnvalue_2 false true)
        (Default|CreateLobbyMenu _asbp_my_player_controler)
        (for _array_element _all_playercontrolers
          (Default|CreatePlayerList _array_element _all_playercontrolers))
        (Default|InitialSetup _asbp_my_player_controler)))
    (else
      (bind _asbp_my_player_controler_2 (Utilities|Casting|CastToBP_MyPlayerControler NewPlayer))
      (Default|OCKickPlayer _asbp_my_player_controler_2 "Gra działa"))))

(event EventOnLogout
  (params (ExitingController :type Controller%20Object%20Reference))
  (bind _all_playercontrolers (Variables|Default|GetAll_PlayerControlers))
  ;[1 1 1] Wyjscie gracza
  (bind _asbp_my_player_controler (Utilities|Casting|CastToBP_MyPlayerControler ExitingController))
  (Utilities|Array|RemoveIndex (Variables|Default|GetIsPlayerRedy) (Utilities|Array|FindItem _all_playercontrolers _asbp_my_player_controler))
  (Utilities|Array|RemoveIndex _all_playercontrolers (Utilities|Array|FindItem _all_playercontrolers _asbp_my_player_controler))
  (if (Variables|Default|Getgra)
    (for _array_element _all_playercontrolers
      (Default|CreatePlayerList _array_element _all_playercontrolers))
    (CallFunction|UpdateLobby true true)))

(fn ConstructionScript)

(fn KickPlayer
  (params (id_player :type Integer))
  (Default|OCKickPlayer (Utilities|Array|Get(acopy) (Variables|Default|GetAll_PlayerControlers) id_player)))