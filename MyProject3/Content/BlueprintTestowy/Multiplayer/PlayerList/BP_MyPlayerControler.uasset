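; Player controller for the multiplayer lobby and match flow, handling the lobby menu, player list, ready states, kicks and end results.
; It loads the saved profile and passes it, along with ready changes and scores, to BP_Mygamemode1 through server-named events.
; Update events refresh the WBPoczekalnia lobby widget.
; It also streams the plansza1_multi level in and out, caches results in the game instance and shows a post-game waiting screen.
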(event Custom|OC_KickPlayer
  (params (Wiadomosć :type String))
  ;[0.2001 1 0] LobbyFunkcej
  ;;[1 1 1] Wyżucenie gracza
  (|DestroySession self
    (:OnSuccess
      (Game|OpenLevel(byObjectReference) "/Game/state_level.state_level" true "listen")
      (Development|PrintString Wiadomosć))))

(event Custom|cancel
  ;[1 1 1] Zmiana serwera + czas
  ;;[1 1 1] Pozostawione funkcje poto by się nie wykszaczył kod
  (Default|CancelCountdown (Variables|Default|GetArray%20Element)))

(event Custom|Initial_Setup
  ;[0.2001 1 0] LobbyFunkcej
  ;;[1 1 1] Załadowanie informacji klienta
  (CallFunction|LoadSavedProfile)
  (CallFunction|ServerUpdateLobby (Variables|Default|GetPlayer_Profile_Info)))

(event Custom|Server_UpdateLobby
  (params (PlayerProfile :type S%20Player%20Profile%20Structure))
  ;[0.2001 1 0] LobbyFunkcej
  ;;[1 1 1] Update Lobby Clienta
  (Variables|Default|SetPlayer_Profile_Info PlayerProfile)
  (bind _asbp_mygamemode_1 (Utilities|Casting|CastToBP_Mygamemode1 (Game|GetGameMode)))
  (Default|UpdateLobby _asbp_mygamemode_1 true true))

(event Custom|Server_UpdatePlayerReady
  (params (IsReady :type Boolean))
  ;[0.2001 1 0] LobbyFunkcej
  ;;[1 1 1] Ustawienie Ready player
  (bind _asbp_mygamemode_1 (Utilities|Casting|CastToBP_Mygamemode1 (Game|GetGameMode)))
  (Default|SetPlayerReady _asbp_mygamemode_1 self IsReady))

(event Custom|UpdatePlayerReady
  (params (IsPlayerRedy :type Array%20of%20Booleans))
  (bind _wb_poczekalnia (Variables|Default|GetWB_Poczekalnia))
  ;[0.2001 1 0] LobbyFunkcej
  ;;[1 1 1] Update Ready
  (Utilities|IsValid _wb_poczekalnia
    (:Is%20Valid
      (Default|UpdatePlayersReady _wb_poczekalnia IsPlayerRedy))))

(event Custom|Create_end_playlist
  (params (NewParam :type Array%20of%20BP%20My%20Player%20Controler%20Object%20References) (SerwerPlayer%20controler :type BP%20My%20Player%20Controler%20Object%20Reference) (tabela_wyników :type Array%20of%20S%20Tabela%20Wyników%20Structures))
  ;[0 0.4326 1] Wysłanie wyników end
  ;;[1 1 1] Stwożenie listy wyników
  (Default|UpdateWidgetEnd (Variables|Default|GetWB_Poczekalnia) NewParam SerwerPlayer%20controler tabela_wyników))

(event Custom|Change_mape
  ;[0 0.4326 1] Wysłanie wyników end
  (Game|UnloadStreamLevel(byName) "plansza1_multi" false))

(event Custom|pobranie_z_instancji
  ;[0 0.4326 1] Wysłanie wyników end
  (bind _asbp_game_instance_2 (Utilities|Casting|CastToBp_GameInstance2 (Game|GetGameInstance)))
  (bind _output_get (Variables|Default|SetEnd_wynik (Variables|/Game/BlueprintTestowy/SaveData/Bp_GameInstance2.Bp_GameInstance2_C|GetWynik_end _asbp_game_instance_2)))
  (Development|PrintString (Utilities|String|ToString(Float) (Utilities|Struct|BreakS_Tabela_Wyników _output_get)) true true "(R=1.000000,G=0.000000,B=0.738211,A=1.000000)" 12.0))

(event Custom|Wysłanie_wyników
  (params (Tabela_wyników :type S%20Tabela%20Wyników%20Structure))
  (bind _self self)
  ;[0 0.4326 1] Wysłanie wyników end
  ;;[1 1 1] wysłanie wyniku
  (Variables|Default|SetEnd_wynik Tabela_wyników)
  (bind _asbp_game_instance_2 (Utilities|Casting|CastToBp_GameInstance2 (Game|GetGameInstance)))
  (Variables|/Game/BlueprintTestowy/SaveData/Bp_GameInstance2.Bp_GameInstance2_C|SetWynik_end _asbp_game_instance_2 Tabela_wyników)
  (CallFunction|WysłanieDoSerwera _self _self Tabela_wyników))

(event Custom|Chainge_level
  (params (muzyka :type Opcje%20Muzyki%20Structure))
  ;[1 1 1] Zmiana serwera + czas
  ;;[1 1 1] Zmiana poziomu dla klienta
  (bind _asbp_game_instance_2 (Utilities|Casting|CastToBp_GameInstance2 (Game|GetGameInstance)))
  (Variables|/Game/BlueprintTestowy/SaveData/Bp_GameInstance2.Bp_GameInstance2_C|Setmuzyka _asbp_game_instance_2 muzyka)
  (Default|SetReturntoGameMode _asbp_game_instance_2)
  (Viewport|RemoveAllWidgets)
  (Game|LoadStreamLevel(byName) "plansza1_multi" true))

(event Custom|set_time
  (params (NewParam :type Integer))
  ;[1 1 1] Zmiana serwera + czas
  ;;[1 1 1] Pozostawione funkcje poto by się nie wykszaczył kod
  (Default|StartCountdown (Variables|Default|GetArray%20Element) NewParam))

(event Custom|CreateLobbyMenu
  ;[0.2001 1 0] LobbyFunkcej
  ;;[1 1 1] Stawożenie menu multi playera
  (CallFunction|UiShowLobbyMenu))

(event Custom|wysłanie%20do%20serwera
  (params (ThisPlayerControler :type BP%20My%20Player%20Controler%20Object%20Reference) (End_wynik :type S%20Tabela%20Wyników%20Structure))
  ;[0 0.4326 1] Wysłanie wyników end
  ;;[1 1 1] Wysłanie do serwera po zakończonej rozgrywce
  (Variables|Default|SetEnd_wynik End_wynik)
  (bind _asbp_mygamemode_1 (Utilities|Casting|CastToBP_Mygamemode1 (Game|GetGameMode)))
  (Default|WysłanieDoSerwera _asbp_mygamemode_1 ThisPlayerControler))

(event Custom|Update_Player_Names
  (params (PlayerProfiles :type Array%20of%20S%20Player%20Profile%20Structures))
  (bind _wb_poczekalnia (Variables|Default|GetWB_Poczekalnia))
  ;[0.2001 1 0] LobbyFunkcej
  ;;[1 1 1] Update Names
  (Utilities|IsValid _wb_poczekalnia
    (:Is%20Valid
      (Default|ClearPlayerNames _wb_poczekalnia)
      (Default|UpdatePlayerNamesLobby _wb_poczekalnia PlayerProfiles))))

(event Custom|Ekran_poczekalni_po_rozgrywce
  ;[0 0.4326 1] Wysłanie wyników end
  ;;[1 1 1] Wywołanie poczekalni dla graczy.
  (Viewport|RemoveAllWidgets)
  (bind _returnvalue (UserInterface|CreateWidget "/Game/BlueprintTestowy/Multiplayer/UI_Końcowy/WP_Waiting_screen.WP_Waiting_screen_C" self))
  (UserInterface|Viewport|AddtoViewport _returnvalue 0))

(event Custom|CreatePlayerList
  (params (NewParam :type Array%20of%20BP%20My%20Player%20Controler%20Object%20References))
  ;[0.2001 1 0] LobbyFunkcej
  ;;[1 1 1] Stwożenie listy wszystkich playerów
  (Default|UpdateWidgetLobby (Variables|Default|GetWB_Poczekalnia) NewParam))

(event EventBeginPlay
  ;[0.2001 1 0] LobbyFunkcej
  ;;[1 1 1] Pokazanie kursora
  (if (Pawn|IsLocalController)
    (Variables|Default|SetbShowMouseCursor true)
    (Input|SetInputModeUIOnly self 0 "DoNotLock" false)))

(fn ConstructionScript)

(fn Update
  (params (NewParam :type Integer) (InputPin :type Array%20of%20Player%20State%20Object%20References)))

(fn UiShowLobbyMenu
  (Viewport|RemoveAllWidgets)
  (Utilities|IsValid (Variables|Default|GetWB_Poczekalnia)
    (:Is%20Valid
      _)
    (:Is%20Not%20Valid
      (bind _returnvalue (Game|ConstructObjectfromClass self "/Game/BlueprintTestowy/Multiplayer/Widget_poczekalnia.Widget_poczekalnia_C"))
      (Variables|Default|SetWB_Poczekalnia _returnvalue)))
  (UserInterface|Viewport|AddtoViewport (Variables|Default|GetWB_Poczekalnia) 0)
  (return))

(fn LoadSavedProfile
  (bind _returnvalue (SaveGame|DoesSaveGameExist (LocalVariables|GetLcl_SlotName)))
  (if _returnvalue
    _
    (else
      (bind _returnvalue_2 (SaveGame|CreateSaveGameObject "/Game/BlueprintTestowy/SaveData/SG_PlayerProfile.SG_PlayerProfile_C"))
      (SaveGame|SaveGametoSlot _returnvalue_2 (LocalVariables|GetLcl_SlotName))))
  (bind _returnvalue_3 (SaveGame|LoadGamefromSlot (LocalVariables|GetLcl_SlotName)))
  (bind _assg_player_profile (Utilities|Casting|CastToSG_PlayerProfile _returnvalue_3))
  (Variables|Default|SetPlayer_Profile_Info (Variables|/Game/BlueprintTestowy/SaveData/SG_PlayerProfile.SG_PlayerProfile_C|GetPlayerProfile _assg_player_profile))
  (return))

(fn CreateWidgetSerwer
  (Viewport|RemoveAllWidgets)
  (bind _returnvalue (UserInterface|CreateWidget "/Game/BlueprintTestowy/Multiplayer/UI_Końcowy/Testowy_UI.Testowy_UI_C" self))
  (UserInterface|Viewport|AddtoPlayerScreen _returnvalue))