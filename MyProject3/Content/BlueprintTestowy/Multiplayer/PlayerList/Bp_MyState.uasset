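; Multiplayer game state for a waiting-room player list, storing player controllers and states through an update event.
; PlayerReference finds a player's controller by PlayerArray index and passes its EveryOneRedy value to the player-list widget with the matching ID.
; Both OnRep functions only loop over waiting-room widgets without acting.
; Their server-side ready checks, which would switch countdowns between 10 and 30 and relay player readiness, are disconnected.
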(event Custom|Update_player_list
  (params (NewParam :type Array%20of%20BP%20My%20Player%20Controler%20Object%20References))
  (Variables|Default|SetAll_Player_Controller NewParam)
  (Variables|Default|SetAll_Player_State (Variables|Default|GetPlayerArray)))

(fn ConstructionScript)

(fn OnRepAllPlayerState
  (bind _foundwidgets (Widget|GetAllWidgetsOfClass "/Game/BlueprintTestowy/Multiplayer/Widget_poczekalnia.Widget_poczekalnia_C" false))
  (for _array_element _foundwidgets
    _))

(fn PlayerReference
  (params (int :type Integer))
  (bind _asbp_my_player_controler (Utilities|Casting|CastToBP_MyPlayerControler (Game|GetPlayerController (Utilities|Array|Get(acopy) (Variables|Default|GetPlayerArray) int))))
  (bind _foundwidgets (Widget|GetAllWidgetsOfClass "/Game/BlueprintTestowy/Multiplayer/PlayerList/WP_Player_list_widget.WP_Player_list_widget_C" true))
  (for _array_element _foundwidgets
    (if (== int (Variables|/Game/BlueprintTestowy/Multiplayer/PlayerList/WP_Player_list_widget.WP_Player_list_widget_C|GetPlayerID _array_element))
      (Default|ReturnEvent _array_element (Variables|/Game/BlueprintTestowy/Multiplayer/PlayerList/BP_MyPlayerControler.BP_MyPlayerControler_C|GetEvery_One_Redy _asbp_my_player_controler)))))

(fn OnRepAllPlayerController
  (bind _foundwidgets (Widget|GetAllWidgetsOfClass "/Game/BlueprintTestowy/Multiplayer/Widget_poczekalnia.Widget_poczekalnia_C" false))
  (for _array_element _foundwidgets
    _))